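; BPC_Inventory is an inventory component that tracks item quantities by name in the InventoryItems map and caches its owner on BeginPlay.
; Adding sums quantities for items already held and prints new entries; removal decrements a positive count and reports success.
; Both operations assign InventoryItems a fresh single-entry MakeMap instead of editing it, so each successful write discards all other items.
; Entries that reach zero remain as keys.
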(event `self.ReceiveBeginPlay`
  (set `self.OwnerActor` (`self.GetOwner`)))

(fn `AddItemToInventory`
  (params (ItemName :type String) (Quantity :type Integer))
  (locals (LocalItem :type String) (LocalQuantity :type Integer))
  (bind _localitem (`local.LocalItem`))
  (bind _localquantity (`local.LocalQuantity`))
  (set `local.LocalItem` ItemName)
  (set `local.LocalQuantity` Quantity)
  (bind _founditem (`self.CheckItemInInventory` ItemName))
  (if _founditem
    (set `self.InventoryItems` (`|MakeMap` (`local.LocalItem`) (+ (`local.LocalQuantity`) (`BlueprintMapLibrary.Map_Find` (`self.InventoryItems`) (`local.LocalItem`)))))
    (else
      (set `self.InventoryItems` (`|MakeMap` _localitem _localquantity))
      (`KismetSystemLibrary.PrintString` _localitem)
      (`KismetSystemLibrary.PrintString` (`KismetStringLibrary.Conv_IntToString` _localquantity)))))

(fn `CheckItemInInventory`
  (params (ItemName :type String))
  (returns (FoundItem :type Boolean))
  (locals (LocalItemName :type String))
  (set `local.LocalItemName` ItemName)
  (bind _keys (`BlueprintMapLibrary.Map_Keys` (`self.InventoryItems`)))
  (return (`KismetArrayLibrary.Array_Contains` _keys (`local.LocalItemName`))))

(fn `RemoveItemFromInventory`
  (params (ItemToRemove :type String))
  (returns (Success :type Boolean))
  (locals (LocalItemToRemove :type String))
  (bind (_value _returnvalue) (`BlueprintMapLibrary.Map_Find` (`self.InventoryItems`) ItemToRemove))
  (set `local.LocalItemToRemove` ItemToRemove)
  (if _returnvalue
    (if (> _value 0)
      (set `self.InventoryItems` (`|MakeMap` (`local.LocalItemToRemove`) (- _value 1)))
      (return true)
      (else
        (return false)))
    (else
      (return false))))