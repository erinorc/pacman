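; BP_MonsterController is the monster's AI controller, running the BT_Monster behavior tree on possession.
; At BeginPlay it caches the locations of all BP_PatrolPoint actors in the level and exposes them through GetPatrolPoints.
; Its AIPerception update only prints a "Seen Player" debug message for updated third-person character actors, without checking whether they were sensed or lost.
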(event `self.ReceivePossess`
  (params (PossessedPawn :type "Pawn Object Reference"))
  (`self.RunBehaviorTree` "/Game/Blueprints/AI/BT_Monster.BT_Monster"))

(event `self.ReceiveBeginPlay`
  (bind _outactors (`GameplayStatics.GetAllActorsOfClass` "/Game/Blueprints/AI/BP_PatrolPoint.BP_PatrolPoint_C"))
  (for _array_element _outactors
    (`KismetArrayLibrary.Array_Add` (`self.PatrolPoints`) (`self.K2_GetActorLocation` _array_element))))

(event `self.AIPerception.OnPerceptionUpdated`
  (params (UpdatedActors :type "Array of Actor Object Reference (by ref)"))
  (for _array_element UpdatedActors
    (cast `/Game/ThirdPerson/Blueprints/BP_ThirdPersonCharacter` _array_element)
    (`KismetSystemLibrary.PrintString` "Seen Player")))

(fn `GetPatrolPoints`
  (returns (PatrolPointLocations :type "Array of Vector Structure"))
  (return (`self.PatrolPoints`)))

(fn `UserConstructionScript`)