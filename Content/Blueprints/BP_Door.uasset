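; BP_Door is an interactable swinging door that can be locked and can require a key.
; Interact opens an unlocked door, or consumes a "Key" from the player's BPCInventory to unlock and open it.
; A Timeline offsets yaw from the rotation saved at BeginPlay, with optional delayed auto-close by reversing it.
; Open and close sounds play at the door, but locked or failed-removal sounds play at world origin.
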(event `self.ReceiveBeginPlay`
  (set `self.StartRotation` (`SceneComponent.K2_GetComponentRotation` (`self.Door`))))

(event `/Game/Blueprints/BPI_Interactable.Interact`
  (if (`self.Locked`)
    (if (`self.NeedsKey`)
      (bind _playerref (`/Game/Blueprints/BPF_GetPlayer.GetPlayerCharacter`))
      (bind _bpc_inventory (`/Game/ThirdPerson/Blueprints/BP_ThirdPersonCharacter.BPC_Inventory` _playerref))
      (bind _founditem (`/Game/Blueprints/Inventory/BPC_Inventory.CheckItemInInventory` _bpc_inventory "Key"))
      (if _founditem
        (bind _success (`/Game/Blueprints/Inventory/BPC_Inventory.RemoveItemFromInventory` _bpc_inventory "Key"))
        (if _success
          (set `self.Locked` false)
          (set `self.NeedsKey` false)
          (`GameplayStatics.PlaySoundAtLocation` "/Game/SmallSoundKit/SSKCue/DoorsCue/Drs_Wood_Door_Open_01_Cue.Drs_Wood_Door_Open_01_Cue" (`self.K2_GetActorLocation`) (struct) 4.0 1.0 0.0 null null null null :!label _label)
          (bind (_direction _newtrack_0) (`Timeline|Timeline` :!label _label_2)
            (:`Update`
              (`SceneComponent.K2_SetWorldRotation` (`self.Door`) (`KismetMathLibrary.MakeRotator` (.roll (`self.StartRotation`)) (.pitch (`self.StartRotation`)) (+ (.yaw (`self.StartRotation`)) _newtrack_0)) false false))
            (:`Finished`
              (if (`self.AutoClose`)
                (`KismetSystemLibrary.Delay` (`self.CloseDelay`))
                (`self.CloseDoor`))))
          (else
            (`GameplayStatics.PlaySoundAtLocation` "/Game/SmallSoundKit/SSKCue/DoorsCue/Drs_Wood_Door_Close_01_Cue.Drs_Wood_Door_Close_01_Cue" (0.0 0.0 0.0) (struct) 2.0 1.0 0.0 null null null null))))
      (else
        (`GameplayStatics.PlaySoundAtLocation` "/Game/SmallSoundKit/SSKCue/DoorsCue/Drs_Wood_Door_Close_01_Cue.Drs_Wood_Door_Close_01_Cue" (0.0 0.0 0.0) (struct) 2.0 1.0 0.0 null null null null)))
    (else
      (goto _label))))

(event `CloseDoor`
  (`GameplayStatics.PlaySoundAtLocation` "/Game/SmallSoundKit/SSKCue/DoorsCue/Drs_Wood_Door_Close_01_Cue.Drs_Wood_Door_Close_01_Cue" (`self.K2_GetActorLocation`) (struct) 2.0 1.0 0.0 null null null null)
  (goto _label_2 :!via `Reverse`))

(fn `UserConstructionScript`)